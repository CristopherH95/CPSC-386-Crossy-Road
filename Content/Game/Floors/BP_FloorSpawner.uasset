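; Floor spawner actor that builds a chained track of BP_Grass floors, laying an initial run on BeginPlay.
; Each new floor spawns at the newest one's SpawnPoint, receives a reference to this spawner, and joins the Floors array.
; Limit-enforced spawns increment a counter that, at its threshold, destroys only the oldest floor and resets.
; SpawnFloorAtSpawnPoint's DisableLimitEnforcement input feeds EnforceLimit directly, so true enables the limit despite its name.
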(event EventBeginPlay
  (CallFunction|SpawnInitialFloors))

(event Collision|EventActorBeginOverlap
  (params (OtherActor :type Actor%20Object%20Reference)))

(event EventTick
  (params (DeltaSeconds :type Float%20%28single-precision%29)))

(fn ConstructionScript)

(fn SpawnFloor
  (params (SpawnLocation :type Vector) (EnforceLimit :type Boolean))
  (bind _floors (Variables|Default|GetFloors))
  (bind _returnvalue (Game|SpawnActorfromClass "/Game/Game/Floors/BP_Grass.BP_Grass_C" (Math|Transform|MakeTransform SpawnLocation "0, 0, 0" "1,1,1") "Undefined" 0 0))
  (bind _output_get (Variables|Default|SetNewestFloor _returnvalue))
  (Variables|/Game/Game/Floors/BP_Floor.BP_Floor_C|SetFloorSpawner _output_get self)
  (Utilities|Array|Add (Variables|Default|GetFloors) _output_get)
  (if EnforceLimit
    (bind _result (Math|Integer|IncrementInt (Variables|Default|GetFloorCounter))
      (:%20%20
        (if (>= _result 10)
          (Actor|DestroyActor (Utilities|Array|Get(acopy) _floors))
          (Utilities|Array|RemoveIndex _floors)
          (Variables|Default|SetFloorCounter 0))))))

(fn SpawnFlooratSpawnPoint
  (params (DisableLimitEnforcement :type Boolean))
  (CallFunction|SpawnFloor (Transformation|GetWorldLocation (Variables|/Game/Game/Floors/BP_Floor.BP_Floor_C|GetSpawnPoint (Variables|Default|GetNewestFloor))) DisableLimitEnforcement))

(fn SpawnInitialFloors
  (for _index (range 0 4)
    (Utilities|IsValid (Variables|Default|GetNewestFloor)
      (:Is%20Valid
        (CallFunction|SpawnFlooratSpawnPoint true))
      (:Is%20Not%20Valid
        (CallFunction|SpawnFloor "400.000000, 0,20.000000" false)))))