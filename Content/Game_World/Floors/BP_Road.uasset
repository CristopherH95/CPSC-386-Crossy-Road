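; BP_Road is a road floor tile that spawns a car on itself at BeginPlay.
; A random choice picks one of two spawn points with opposite yaw, and SpawnVehicle creates a BP_Car there with a set speed and direction.
; It spawns only while no valid vehicle is stored, then starts a five-second one-shot timer.
; Two kill volumes destroy any BP_Vehicle that overlaps them.
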(event OnComponentBeginOverlap(VehicleKill0)
  (params (OverlappedComponent :type Primitive%20Component%20Object%20Reference) (OtherActor :type Actor%20Object%20Reference) (OtherComp :type Primitive%20Component%20Object%20Reference) (OtherBodyIndex :type Integer) (bFromSweep :type Boolean) (SweepResult :type Hit%20Result%20Structure%20%28by%20ref%29))
  (bind _asbp_vehicle (Utilities|Casting|CastToBP_Vehicle OtherActor))
  (Actor|DestroyActor _asbp_vehicle))

(event OnComponentBeginOverlap(VehicleKill1)
  (params (OverlappedComponent :type Primitive%20Component%20Object%20Reference) (OtherActor :type Actor%20Object%20Reference) (OtherComp :type Primitive%20Component%20Object%20Reference) (OtherBodyIndex :type Integer) (bFromSweep :type Boolean) (SweepResult :type Hit%20Result%20Structure%20%28by%20ref%29))
  (bind _asbp_vehicle (Utilities|Casting|CastToBP_Vehicle OtherActor))
  (Actor|DestroyActor _asbp_vehicle))

(event EventBeginPlay
  (|CallParentFunction)
  (Variables|Default|SetVehicleSpawnChoice (Math|Random|RandomInteger 2))
  (Variables|Default|SetSpeedScale 5.0)
  (CallFunction|SpawnVehicle))

(event Collision|EventActorBeginOverlap
  (params (OtherActor :type Actor%20Object%20Reference))
  (|CallParentFunction OtherActor) ; This node is disabled and will not be called.\nDrag off pins to build functionality.
)

(event EventTick
  (params (DeltaSeconds :type Float%20%28single-precision%29))
  (|CallParentFunction DeltaSeconds) ; This node is disabled and will not be called.\nDrag off pins to build functionality.
)

(fn ConstructionScript
  (|CallParentFunction))

(fn OffsetLocation
  (params (Original :type Vector) (OffsetX :type Float%20%28single-precision%29) (OffsetY :type Float%20%28single-precision%29) (OffsetZ :type Float%20%28single-precision%29))
  (bind (_x _y _z) (Math|Vector|BreakVector Original))
  (return (Math|Vector|MakeVector (+ _x OffsetX) (+ _y OffsetY) (+ _z OffsetZ))))

(fn SpawnVehicle
  (Utilities|IsValid (Variables|Default|GetVehicle)
    (:Is%20Not%20Valid
      (if (> (Variables|Default|GetVehicleSpawnChoice) 0)
        (bind _newlocation (CallFunction|OffsetLocation (Transformation|GetWorldLocation (Variables|Default|GetVehicleSpawn1)) -5e+01 0.0 0.0))
        (bind _returnvalue (Game|SpawnActorfromClass "/Game/Game_World/Vehicles/BP_Car.BP_Car_C" (Math|Transform|MakeTransform _newlocation "0,-90.000000, 0" "1,1,1") "Undefined" 0 0))
        (Variables|/Game/Game_World/Vehicles/BP_Vehicle.BP_Vehicle_C|SetDirection _returnvalue -1.0)
        (Variables|/Game/Game_World/Vehicles/BP_Vehicle.BP_Vehicle_C|SetSpeed _returnvalue (Variables|Default|GetSpeedScale))
        (Variables|Default|SetVehicle _returnvalue)
        (Utilities|Time|SetTimerbyEvent (EventDispatchers|CreateEvent :!event SpawnVehicle) 5.0)
        (else
          (bind _newlocation_2 (CallFunction|OffsetLocation (Transformation|GetWorldLocation (Variables|Default|GetVehicleSpawn0)) -5e+01 0.0 0.0))
          (bind _returnvalue_2 (Game|SpawnActorfromClass "/Game/Game_World/Vehicles/BP_Car.BP_Car_C" (Math|Transform|MakeTransform _newlocation_2 "0,90.000000, 0" "1,1,1") "Undefined" 0 0))
          (Variables|/Game/Game_World/Vehicles/BP_Vehicle.BP_Vehicle_C|SetDirection _returnvalue_2 -1.0)
          (Variables|/Game/Game_World/Vehicles/BP_Vehicle.BP_Vehicle_C|SetSpeed _returnvalue_2 (Variables|Default|GetSpeedScale))
          (Variables|Default|SetVehicle _returnvalue_2)
          (Utilities|Time|SetTimerbyEvent (EventDispatchers|CreateEvent :!event SpawnVehicle) 5.0))))))