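; BP_Chicken is a controllable chicken character with camera-relative movement and jumping.
; Move_X and Move_Y drive forward and sideways movement along the control rotation's yaw, and the jump fires when the Jump input is released.
; The construction script caches the first BP_GameManager it finds, unused in these graphs, and sets the character to rotate toward its movement direction.
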(event EventBeginPlay)

(event Collision|EventActorBeginOverlap
  (params (OtherActor :type Actor%20Object%20Reference)))

(event EventTick
  (params (DeltaSeconds :type Float%20%28single-precision%29)))

(event Input|ActionEvents|InputActionJump
  (params (Key :type Key%20Structure))
  (:Released
    (Character|Jump)))

(event Input|AxisEvents|InputAxisMove_X
  (params (AxisValue :type Float%20%28single-precision%29))
  (Pawn|Input|AddMovementInput (Math|Vector|GetForwardVector (Math|Rotator|MakeRotator 0.0 0.0 (.Yaw (Math|Rotator|BreakRotator (Pawn|GetControlRotation :!class /Script/Engine.Pawn))))) AxisValue false))

(event Input|AxisEvents|InputAxisMove_Y
  (params (AxisValue :type Float%20%28single-precision%29))
  (Pawn|Input|AddMovementInput (Math|Vector|GetRightVector (Math|Rotator|MakeRotator 0.0 0.0 (.Yaw (Math|Rotator|BreakRotator (Pawn|GetControlRotation :!class /Script/Engine.Pawn))))) AxisValue false))

(fn ConstructionScript
  (bind _outactors (Actor|GetAllActorsOfClass "/Game/BP_GameManager.BP_GameManager_C"))
  (Variables|Default|SetGameManager (Utilities|Array|Get(acopy) _outactors))
  (Variables|/Script/Engine.CharacterMovementComponent|SetbOrientRotationToMovement (Variables|Character|GetCharacterMovement) true))