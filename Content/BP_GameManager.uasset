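; BP_GameManager is a pawn that manages score and acts as the player's view in a chicken game, moving steadily along world +X until the chicken is hit.
; BeginPlay creates the score widget, makes itself the view target and caches the first BP_Chicken as Player.
; Tick feeds constant movement input, consumes it immediately and applies it as a swept, per-frame offset without delta-time scaling.
; IncrementScore raises the score and refreshes the widget.
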(event EventBeginPlay
  (bind _returnvalue (UserInterface|CreateWidget "/Game/UI/WBP_ScoreTracker.WBP_ScoreTracker_C"))
  (UserInterface|Viewport|AddtoViewport _returnvalue 0)
  (Variables|/Game/UI/WBP_ScoreTracker.WBP_ScoreTracker_C|SetGameManager _returnvalue self)
  (Variables|Default|SetScoreWidget _returnvalue)
  (Variables|Default|SetbFindCameraComponentWhenViewTarget true)
  (Game|Player|SetViewTargetwithBlend (Game|GetPlayerController 0) self 0.0 "VTBlend_Linear" 0.0 false)
  (bind _outactors (Actor|GetAllActorsOfClass "/Game/Chicken_Assets/BP_Chicken.BP_Chicken_C"))
  (Variables|Default|SetPlayer (Utilities|Array|Get(acopy) _outactors)))

(event Collision|EventActorBeginOverlap
  (params (OtherActor :type Actor%20Object%20Reference)))

(event EventTick
  (params (DeltaSeconds :type Float%20%28single-precision%29))
  (if (not (Variables|/Game/Chicken_Assets/BP_Chicken.BP_Chicken_C|GetHit (Variables|Default|GetPlayer)))
    (Pawn|Input|AddMovementInput "1.000000, 0, 0" 1.0 false)
    (bind _returnvalue (Class|Pawn|ConsumeMovementInputVector))
    (Transformation|AddActorLocalOffset _returnvalue true false)))

(fn ConstructionScript)

(fn IncrementScore
  (Variables|Default|SetScore (+ (Variables|Default|GetScore) 1))
  (Default|UpdateScoreCounter (Variables|Default|GetScoreWidget)))